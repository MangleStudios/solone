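; Radius measuring tool that scales to a set radius and labels the resulting circle's diameter and circumference.
; All work runs in the construction script, so there is no runtime logic.
; It scales from Radius and a multiplier, then derives both values from the distance between two world locations.
; Text color and each readout's visibility are configurable; diameter displays divided by 100, circumference in raw units.
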(event EventBeginPlay)

(event Collision|EventActorBeginOverlap
  (params (OtherActor :type Actor%20Object%20Reference)))

(event EventTick
  (params (DeltaSeconds :type Float%20%28single-precision%29)))

(fn ConstructionScript
  (bind _returnvalue (Transformation|GetWorldLocation))
  (bind _returnvalue_2 (Transformation|GetWorldLocation))
  (bind _radius (Variables|ToolProperties|GetRadius))
  (bind _scale_multiplier (Variables|Misc|GetScale_Multiplier))
  (bind _returnvalue_3 (- _returnvalue _returnvalue_2))
  (bind _returnvalue_4 (/ _radius 1e+02))
  (bind _returnvalue_5 (Math|Vector|VectorLength _returnvalue_3))
  (bind _returnvalue_6 (* _returnvalue_4 _scale_multiplier))
  (bind _returnvalue_7 (* _returnvalue_5 2.0))
  (bind _returnvalue_8 (* _returnvalue_6 0.02))
  (Rendering|Components|TextRender|SetTextRenderColor (Variables|Default|GetDiameterAmount) (Math|Conversions|ToColor(LinearColor) (Variables|ToolProperties|GetText%20Color)))
  (Transformation|SetWorldScale3D (Math|Vector|MakeVector _returnvalue_8 _returnvalue_8 0.01))
  (Variables|Default|SetDiameter _returnvalue_7)
  (Variables|Default|SetCircumference (Math|Float|MultiplybyPi _returnvalue_7))
  (Rendering|Components|TextRender|SetText (Utilities|String|ToString(Float) (Variables|Default|GetCircumference)))
  (Rendering|Components|TextRender|SetText (Utilities|String|ToString(Float) (/ (Variables|Default|GetDiameter) 1e+02)))
  (if (Variables|ToolProperties|GetDisplayDiameter)
    _
    (else
      (Rendering|ToggleVisibility false)
      (Rendering|ToggleVisibility false)))
  (if (not (Variables|ToolProperties|GetDisplayCircumference))
    (Rendering|ToggleVisibility false)
    (Rendering|ToggleVisibility false)))