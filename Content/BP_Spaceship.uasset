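; BP_Spaceship is a player-controlled spaceship with switchable cockpit and external camera views.
; Two input actions toggle between the 1stPersonCam and ExtCam components by activating one and deactivating the other.
; The Left and Up axes feed controller yaw and pitch input.
; The Thust axis event activates the Booster component regardless of axis value, with no deactivation or movement logic in this graph.
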(event Input|ActionEvents|InputActionExternalCamera
  (params (Key :type Key%20Structure))
  (:Pressed
    (Components|Activation|Activate (Variables|Default|GetExtCam) false)
    (Components|Activation|Deactivate (Variables|Default|Get1stPersonCam))))

(event Input|ActionEvents|InputActionCockpitCamera
  (params (Key :type Key%20Structure))
  (:Pressed
    (Components|Activation|Activate (Variables|Default|Get1stPersonCam) false)
    (Components|Activation|Deactivate (Variables|Default|GetExtCam))))

(event Input|AxisEvents|InputAxisThust
  (params (AxisValue :type Float%20%28single-precision%29))
  (Components|Activation|Activate (Variables|Default|GetBooster) false))

(event Input|AxisEvents|InputAxisLeft
  (params (AxisValue :type Float%20%28single-precision%29))
  (Pawn|Input|AddControllerYawInput AxisValue))

(event Input|AxisEvents|InputAxisUp
  (params (AxisValue :type Float%20%28single-precision%29))
  (Pawn|Input|AddControllerPitchInput AxisValue))

(fn ConstructionScript)